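; BP_PipeSpline is a spline actor Blueprint that refreshes its bounds on construction; no pipe mesh generation appears here.
; The construction script calls UpdateBounds, then the parent's script.
; ComputeBoundingBox derives a local-space min/max box from the spline points, raising the maximum by a fixed height from GetBoundsVerticalHeight.
; PivotToSplineCenter is an empty stub, and the event graph is inactive.
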(event EventBeginPlay)

(event Collision|EventActorBeginOverlap
  (params (OtherActor :type Actor%20Object%20Reference)))

(event EventTick
  (params (DeltaSeconds :type Float%20%28single-precision%29)))

(fn ConstructionScript
  (Class|ProceduralPipeActor|UpdateBounds)
  (|CallParentFunction))

(fn PivottoSplineCenter)

(fn ComputeBoundingBox
  (bind _spline (Variables|Default|GetSpline))
  (bind _spline_2 (Variables|Default|GetSpline))
  (bind _returnvalue (Spline|GetNumberOfSplinePoints _spline))
  (bind _returnvalue_2 (Spline|GetLocationatSplinePoint _spline_2 0 "Local"))
  (bind _height (CallFunction|GetBoundsVerticalHeight))
  (LocalVariables|Setoffset (Math|Vector|MakeVector 0.0 0.0 _height))
  (LocalVariables|Setminimum _returnvalue_2)
  (LocalVariables|Setmaximum (+ _returnvalue_2 (LocalVariables|Getoffset)))
  (if (> _returnvalue 1)
    (for _index (range 1 (- _returnvalue 1))
      (LocalVariables|Setminimum (Math|Vector|MakeVector (Math|Float|Min(Float) (.X (Math|Vector|BreakVector (Spline|GetLocationatSplinePoint (Variables|Default|GetSpline) _index "Local"))) (.X (Math|Vector|BreakVector (LocalVariables|Getminimum)))) (Math|Float|Min(Float) (.Y (Math|Vector|BreakVector (Spline|GetLocationatSplinePoint (Variables|Default|GetSpline) _index "Local"))) (.Y (Math|Vector|BreakVector (LocalVariables|Getminimum)))) (Math|Float|Min(Float) (.Z (Math|Vector|BreakVector (Spline|GetLocationatSplinePoint (Variables|Default|GetSpline) _index "Local"))) (.Z (Math|Vector|BreakVector (LocalVariables|Getminimum))))))
      (LocalVariables|Setmaximum (Math|Vector|MakeVector (Math|Float|Max(Float) (.x (+ (Spline|GetLocationatSplinePoint (Variables|Default|GetSpline) _index "Local") (LocalVariables|Getoffset))) (.X (Math|Vector|BreakVector (LocalVariables|Getmaximum)))) (Math|Float|Max(Float) (.y (+ (Spline|GetLocationatSplinePoint (Variables|Default|GetSpline) _index "Local") (LocalVariables|Getoffset))) (.Y (Math|Vector|BreakVector (LocalVariables|Getmaximum)))) (Math|Float|Max(Float) (.z (+ (Spline|GetLocationatSplinePoint (Variables|Default|GetSpline) _index "Local") (LocalVariables|Getoffset))) (.Z (Math|Vector|BreakVector (LocalVariables|Getmaximum)))))))
    (return (LocalVariables|Getminimum) (LocalVariables|Getmaximum))))

(fn GetBoundsVerticalHeight
  (return 1e+02))